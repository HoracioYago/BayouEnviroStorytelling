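; Static examinable actor that the player can inspect for a front-side comment, with special instances driving a scripted attic scare.
; When unlocked, interacting flags it as inspected; the attic bed instance then reveals and unlocks the bodies examinable.
; The bodies instance starts hidden, and inspecting it reveals and unlocks the demon and closes the attic door.
; Interface getters report it as static and inspectable, supplying comment, prompt, animation and UI placement data.
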(event `self.ReceiveBeginPlay`
  (if (`self.Bodies`)
    (`self.SetActorHiddenInGame` self true)))

(event `self.Interact`
  (params (Interactor :type "Actor Object Reference"))
  (bind _demonref (`self.DemonRef`))
  (bind _bodiesref (`self.BodiesRef`))
  (if (not (`self.locked?`))
    (set `self.Inspected Static` true)
    (if (`self.isAtticBed?`)
      (`self.SetActorHiddenInGame` _bodiesref false)
      (set `/Game/ExportToBayou/BP_StaticExaminable.locked?` false _bodiesref)
      (set `/Game/ExportToBayou/BP_StaticExaminable.Inspected Static` false _bodiesref)
      (elif (`self.Bodies`)
        (`self.SetActorHiddenInGame` _demonref false)
        (set `/Game/ExportToBayou/BP_Demon.Locked` false _demonref)
        (`/Game/ExportToBayou/BP_AtticStairs.CloseAtticDoor` (`self.AtticStairs`))))))

(event `self.Disengage`
  (params (Interactor :type "Actor Object Reference")))

(event `self.FlipInspect`)

(event `self.TalkedAbout`
  (params (TalkedAbout :type Boolean))
  (set `self.Has Been Commented` TalkedAbout))

(event `self.TalkedAboutBack`
  (params (TalkedAboutBack :type Boolean))
  (set `self.Has Been Commented Back` TalkedAboutBack))

(fn `GetHoldDuration`
  (returns (Duration :type "Float (double-precision)"))
  (return 0.5))

(fn `GetInspectInfo`
  (returns (Name :type Text) (PlayerComment :type Text) (PlayerBackComment :type Text) (UnpinDialogue :type Text) (HasComment :type Boolean) (HasBackComment :type Boolean) (HasBeenCommented :type Boolean) (HasBeenCommentedBack :type Boolean) (`IsDoll?` :type Boolean) (FrontDialogueDuration :type "Float (double-precision)") (BackDialogueDuration :type "Float (double-precision)") (UnpinDialogueDuration :type "Float (double-precision)") (FrontDialogueLine :type "SoundBase Object Reference") (BackDialogueLine :type "SoundBase Object Reference") (UnpinDialogueLine :type "SoundBase Object Reference"))
  (return "" (`self.Player Comment`) "" "" (`self.Has Comment`) false (`self.Has Been Commented`) false false (`self.Front Dialogue Duration`) 0.0 0.0 (`self.Front Dialogue Line`) null null))

(fn `GetInteractionPrompt`
  (returns (Value :type Text))
  (return (select `bool` (`self.isBeingExamined`) :`false` "to open the door" :`true` "to close the door" :!type "Text")))

(fn `GetInteractionType`
  (returns (Type :type "/Game/ExportToBayou/E_InteractionInputType Enum"))
  (return (`self.InputType`)))

(fn `IsBeingInteractedWith?`
  (returns (IsInteracting :type Boolean))
  (return (`self.isBeingExamined`)))

(fn `IsDoll?`
  (returns (Dollness :type Boolean) (`Unpinned?` :type Boolean))
  (return false false))

(fn `isInspectable?`
  (returns (isInspectObject :type Boolean))
  (return true))

(fn `IsInspectedStatic`
  (returns (`IsStatic?` :type Boolean) (InspectedStatic :type Boolean))
  (return true (`self.Inspected Static`)))

(fn `IsLockedDoor?`
  (returns (`LockedDoor?` :type Boolean))
  (return false))

(fn `IsNotDialogueTrigger`
  (returns (NotDialogueTrigger :type Boolean))
  (return true))

(fn `SetAnimation`
  (returns (InteractAnimation :type "AnimMontage Object Reference"))
  (return (`self.InteractAnimation`)))

(fn `SetUI`
  (returns (DrawSize :type "Vector2D Structure") (UILocation :type "Vector Structure"))
  (return (`self.UIDrawSize`) (`SceneComponent.K2_GetComponentLocation` (`self.UI Render Point`))))

(fn `ShouldBeLookedAt`
  (returns (LookAtMe :type Boolean))
  (return true))

(fn `UserConstructionScript`)