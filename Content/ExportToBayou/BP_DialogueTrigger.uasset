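; Dialogue trigger actor that supplies a player comment, dialogue line and duration through what appears to be a shared interaction interface.
; GetInspectInfo packs these three variables with HasComment set and the back-side and unpin fields left empty.
; Other queries return inert defaults, except IsNotDialogueTrigger, which returns true despite the asset's name.
; The event graph and construction script are empty, so the actor triggers nothing itself.
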(fn `GetHoldDuration`
  (returns (Duration :type "Float (double-precision)"))
  (return 0.0))

(fn `GetInspectInfo`
  (returns (Name :type Text) (PlayerComment :type Text) (PlayerBackComment :type Text) (UnpinDialogue :type Text) (HasComment :type Boolean) (HasBackComment :type Boolean) (HasBeenCommented :type Boolean) (HasBeenCommentedBack :type Boolean) (`IsDoll?` :type Boolean) (FrontDialogueDuration :type "Float (double-precision)") (BackDialogueDuration :type "Float (double-precision)") (UnpinDialogueDuration :type "Float (double-precision)") (FrontDialogueLine :type "SoundBase Object Reference") (BackDialogueLine :type "SoundBase Object Reference") (UnpinDialogueLine :type "SoundBase Object Reference"))
  (return "" (`self.Player Comment`) "" "" true false false false false (`self.Dialogue Duration`) 0.0 0.0 (`self.Front Dialogue Line`) null null))

(fn `GetInteractionPrompt`
  (returns (Value :type Text))
  (return ""))

(fn `GetInteractionType`
  (returns (Type :type "/Game/ExportToBayou/E_InteractionInputType Enum"))
  (return "NewEnumerator0"))

(fn `IsBeingInteractedWith?`
  (returns (IsInteracting :type Boolean))
  (return false))

(fn `IsDoll?`
  (returns (Dollness :type Boolean))
  (return false))

(fn `isInspectable?`
  (returns (isInspectObject :type Boolean))
  (return false))

(fn `IsLockedDoor?`
  (returns (`LockedDoor?` :type Boolean))
  (return false))

(fn `IsNotDialogueTrigger`
  (returns (DialogueTrigger :type Boolean))
  (return true))

(fn `SetAnimation`
  (returns (InteractAnimation :type "AnimMontage Object Reference"))
  (return null))

(fn `SetUI`
  (returns (DrawSize :type "Vector2D Structure") (UILocation :type "Vector Structure"))
  (return (0.0 0.0) (0.0 0.0 0.0)))

(fn `ShouldBeLookedAt`
  (returns (LookAtMe :type Boolean))
  (return false))

(fn `UserConstructionScript`)