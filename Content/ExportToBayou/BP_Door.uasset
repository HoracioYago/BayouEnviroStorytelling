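; Interactable hinged door that can be locked, with a scripted creepy opening for scares.
; Interact plays the locked sound, or plays the open sound and toggles the door by running a yaw timeline forward or in reverse.
; CreepyOpen plays a 2D creak, swings the door on its own timeline, then clears Locked.
; Interaction getters supply the open/close prompt, hold duration, UI placement, lock state and a "Huh... Locked" comment.
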(event `self.ReceiveBeginPlay`)

(event `OpenDoor`
  (set `self.isOpen` true)
  (bind (_direction _zrotation) (`Timeline|OpenDoorTimeline` :!label _label)
    (:`Update`
      (`SceneComponent.K2_SetRelativeRotation` (`self.Door`) (`KismetMathLibrary.MakeRotator` 0.0 0.0 _zrotation) false false))))

(event `CloseDoor`
  (set `self.isOpen` false)
  (goto _label :!via `Reverse`))

(event `self.Interact`
  (params (Interactor :type "Actor Object Reference"))
  (if (`self.Locked`)
    (`GameplayStatics.PlaySoundAtLocation` (`self.LockedDoorSound`) (`self.K2_GetActorLocation` self) (struct) 1.0 1.0 0.0 null null null null)
    (else
      (`GameplayStatics.PlaySoundAtLocation` (`self.OpenDoorSound`) (`self.K2_GetActorLocation` self) (struct) 1.0 1.0 0.0 null null null null)
      (if (`self.isOpen`)
        (`self.CloseDoor`)
        (else
          (`self.OpenDoor`))))))

(event `CreepyOpen`
  (`GameplayStatics.PlaySound2D` (`self.CreepyDoorCreak`) 1.0 1.0 0.0 null null)
  (bind (_direction _zrotation _creepy_zrotation) (`Timeline|CreepyOpenDoorTimeline` :!via `PlayFromStart`)
    (:`Update`
      (`SceneComponent.K2_SetRelativeRotation` (`self.Door`) (`KismetMathLibrary.MakeRotator` 0.0 0.0 _creepy_zrotation) false false))
    (:`Finished`
      (set `self.Locked` false))))

(fn `GetHoldDuration`
  (returns (Duration :type "Float (double-precision)"))
  (return 0.5))

(fn `GetInspectInfo`
  (returns (Name :type Text) (PlayerComment :type Text) (PlayerBackComment :type Text) (UnpinDialogue :type Text) (HasComment :type Boolean) (HasBackComment :type Boolean) (HasBeenCommented :type Boolean) (HasBeenCommentedBack :type Boolean) (`IsDoll?` :type Boolean) (FrontDialogueDuration :type "Float (double-precision)") (BackDialogueDuration :type "Float (double-precision)") (UnpinDialogueDuration :type "Float (double-precision)") (FrontDialogueLine :type "SoundBase Object Reference") (BackDialogueLine :type "SoundBase Object Reference") (UnpinDialogueLine :type "SoundBase Object Reference"))
  (return "" "Huh... Locked" "" "" true false false false false 2.0 0.0 0.0 "/Game/Sounds/VoiceLines/Door_Locked.Door_Locked" null null))

(fn `GetInteractionPrompt`
  (returns (Value :type Text))
  (return (select `bool` (`self.isOpen`) :`false` "to open the door" :`true` "to close the door" :!type "Text")))

(fn `GetInteractionType`
  (returns (Type :type "/Game/ExportToBayou/E_InteractionInputType Enum"))
  (return (`self.InputType`)))

(fn `IsBeingInteractedWith?`
  (returns (IsInteracting :type Boolean))
  (return false))

(fn `IsDoll?`
  (returns (Dollness :type Boolean) (`Unpinned?` :type Boolean))
  (return false false))

(fn `isInspectable?`
  (returns (isInspectObject :type Boolean))
  (return false))

(fn `IsInspectedStatic`
  (returns (`IsStatic?` :type Boolean) (InspectedStatic :type Boolean))
  (return false false))

(fn `IsLockedDoor?`
  (returns (`LockedDoor?` :type Boolean))
  (return (`self.Locked`)))

(fn `IsNotDialogueTrigger`
  (returns (NotDialogueTrigger :type Boolean))
  (return true))

(fn `SetAnimation`
  (returns (InteractAnimation :type "AnimMontage Object Reference"))
  (return (`self.InteractAnimation`)))

(fn `SetUI`
  (returns (DrawSize :type "Vector2D Structure") (UILocation :type "Vector Structure"))
  (return (`self.UIDrawSize`) (`SceneComponent.K2_GetComponentLocation` (`self.UI Render Point`))))

(fn `ShouldBeLookedAt`
  (returns (LookAtMe :type Boolean))
  (return true))

(fn `UserConstructionScript`)