(event `self.Interact`
  (params (Interactor :type "Actor Object Reference"))
  (bind (_returnvalue_location _returnvalue_rotation) (`KismetMathLibrary.BreakTransform` (`self.GetTransform`)))
  ;[0 0 0] Interact Logic
  (set `self.isBeingExamined` true)
  (message `/Game/ExportToBayou/BPI_Player.DisableMovement` Interactor true)
  (message `/Game/ExportToBayou/BPI_Player.SetIgnoreLookInput` Interactor true)
  (set `self.OriginalLocation` _returnvalue_location)
  (set `self.OriginalRotation` _returnvalue_rotation)
  (`self.K2_AttachToComponent` self (`PlayerCameraManager.TransformComponent` (`GameplayStatics.GetPlayerCameraManager` 0)) "None" "KeepWorld" "KeepWorld" "KeepWorld" true)
  (`KismetSystemLibrary.MoveComponentTo` (`self.DefaultSceneRoot`) (200.0 0.0 30.0) (struct) false false 0.3)
  (`GameplayStatics.PlaySoundAtLocation` (`self.ExamineSound`) (`self.K2_GetActorLocation` self) (struct) 1.0 1.0 0.0 null null null null)
  (`PrimitiveComponent.SetRenderCustomDepth` (`self.Examinable`) false))

(event `/Game/ExportToBayou/BPI_Interactable.Disengage`
  (params (Interactor :type "Actor Object Reference"))
  ;[0 0 0] Put Back Logic
  (set `self.isBeingExamined` false)
  (message `/Game/ExportToBayou/BPI_Player.DisableMovement` Interactor false)
  (message `/Game/ExportToBayou/BPI_Player.SetIgnoreLookInput` Interactor false)
  (`self.K2_DetachFromActor` self "KeepWorld" "KeepWorld" "KeepWorld")
  (`KismetSystemLibrary.MoveComponentTo` (`self.DefaultSceneRoot`) (`self.OriginalLocation`) (`self.OriginalRotation`) false false 0.3)
  (`GameplayStatics.PlaySoundAtLocation` (`self.ExamineSound`) (`self.K2_GetActorLocation` self) (struct) 1.0 1.0 0.0 null null null null)
  (`PrimitiveComponent.SetRenderCustomDepth` (`self.Examinable`) false))

(event `/Game/ExportToBayou/BPI_Interactable.FlipInspect`
  ;[0 0 0] Flip Logic
  (if (`self.isBeingExamined`)
    (`/Engine/EditorBlueprintResources/StandardMacros.DoOnce` false :!label _label
      (:`Completed`
        (if (`self.IsTurned`)
          (set `self.TargetTurnRotation` (struct))
          (set `self.IsTurned` false)
          (else
            (set `self.TargetTurnRotation` (struct :`Yaw` 180.0))
            (set `self.IsTurned` true)))
        (`KismetSystemLibrary.MoveComponentTo` (`self.DefaultSceneRoot`) (200.0 0.0 30.0) (`self.TargetTurnRotation`))
        (goto _label :!via `Reset`)))))

(event `self.Sphere.OnComponentBeginOverlap`
  (params (OverlappedComponent :type "PrimitiveComponent Object Reference") (OtherActor :type "Actor Object Reference") (OtherComp :type "PrimitiveComponent Object Reference") (OtherBodyIndex :type Integer) (bFromSweep :type Boolean) (SweepResult :type "HitResult Structure (by ref)"))
  ;[0 0 0] Activate / Deactivate Outline on Enter / Exit Overlap
  (if (`KismetSystemLibrary.DoesImplementInterface` OtherActor "/Game/ExportToBayou/BPI_Player.BPI_Player_C")
    (bind (_interactcomponent _capsulecollision) (message `/Game/ExportToBayou/BPI_Player.GetInteractComponentAndFlashlightHitbox` OtherActor))
    (if (== _capsulecollision OtherComp)
      (`PrimitiveComponent.SetRenderCustomDepth` (`self.Examinable`) true))))

(event `self.Sphere.OnComponentEndOverlap`
  (params (OverlappedComponent :type "PrimitiveComponent Object Reference") (OtherActor :type "Actor Object Reference") (OtherComp :type "PrimitiveComponent Object Reference") (OtherBodyIndex :type Integer))
  ;[0 0 0] Activate / Deactivate Outline on Enter / Exit Overlap
  (if (`KismetSystemLibrary.DoesImplementInterface` OtherActor "/Game/ExportToBayou/BPI_Player.BPI_Player_C")
    (bind (_interactcomponent _capsulecollision) (message `/Game/ExportToBayou/BPI_Player.GetInteractComponentAndFlashlightHitbox` OtherActor))
    (if (== _capsulecollision OtherComp)
      (`PrimitiveComponent.SetRenderCustomDepth` (`self.Examinable`) false))))

(event `/Game/ExportToBayou/BPI_Interactable.TalkedAbout`
  (params (TalkedAbout :type Boolean))
  ;[0 0 0] Set if it has been commented on
  (set `self.Has Been Commented` TalkedAbout))

(event `/Game/ExportToBayou/BPI_Interactable.TalkedAboutBack`
  (params (TalkedAboutBack :type Boolean))
  ;[0 0 0] Set if it has been commented on
  (set `self.Has Been Commented Back` TalkedAboutBack))

(fn `GetHoldDuration`
  (returns (Duration :type "Float (double-precision)"))
  (return 0.5))

(fn `GetInspectInfo`
  (returns (Name :type Text) (PlayerComment :type Text) (PlayerBackComment :type Text) (UnpinDialogue :type Text) (HasComment :type Boolean) (HasBackComment :type Boolean) (HasBeenCommented :type Boolean) (HasBeenCommentedBack :type Boolean) (`IsDoll?` :type Boolean) (FrontDialogueDuration :type "Float (double-precision)") (BackDialogueDuration :type "Float (double-precision)") (UnpinDialogueDuration :type "Float (double-precision)") (FrontDialogueLine :type "SoundBase Object Reference") (BackDialogueLine :type "SoundBase Object Reference") (UnpinDialogueLine :type "SoundBase Object Reference"))
  (return (`self.ItemName`) (`self.Player Comment`) (`self.Player Back Comment`) "" (`self.Has Comment`) (`self.Has Back Comment`) (`self.Has Been Commented`) (`self.Has Been Commented Back`) false (`self.Front Dialogue Duration`) (`self.Back Dialogue Duration`) 0.0 (`self.Front Dialogue Line`) (`self.Back Dialogue Line`) (`self.Unpin Dialogue Line`)))

(fn `GetInteractionPrompt`
  (returns (Value :type Text))
  (return (select `bool` (`self.isBeingExamined`) :`false` "to open the door" :`true` "to close the door" :!type "Text")))

(fn `GetInteractionType`
  (returns (Type :type "/Game/ExportToBayou/E_InteractionInputType Enum"))
  (return (`self.InputType`)))

(fn `IsBeingInteractedWith?`
  (returns (IsInteracting :type Boolean))
  (return (`self.isBeingExamined`)))

(fn `IsDoll?`
  (returns (Dollness :type Boolean) (`Unpinned?` :type Boolean))
  (return false false))

(fn `isInspectable?`
  (returns (isInspectObject :type Boolean))
  (return true))

(fn `IsInspectedStatic`
  (returns (`IsStatic?` :type Boolean) (InspectedStatic :type Boolean))
  (return false false))

(fn `IsLockedDoor?`
  (returns (`LockedDoor?` :type Boolean))
  (return false))

(fn `IsNotDialogueTrigger`
  (returns (NotDialogueTrigger :type Boolean))
  (return true))

(fn `SetAnimation`
  (returns (InteractAnimation :type "AnimMontage Object Reference"))
  (return (`self.InteractAnimation`)))

(fn `SetUI`
  (returns (DrawSize :type "Vector2D Structure") (UILocation :type "Vector Structure"))
  (return (`self.UIDrawSize`) (`SceneComponent.K2_GetComponentLocation` (`self.UI Render Point`))))

(fn `ShouldBeLookedAt`
  (returns (LookAtMe :type Boolean))
  (return true))

(fn `UserConstructionScript`)