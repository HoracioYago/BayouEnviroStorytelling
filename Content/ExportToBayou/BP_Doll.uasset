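; BP_Doll is an inspectable doll with a removable pin that dispels its assigned sigil.
; Interacting locks player movement and look, then attaches the doll to the camera for flippable inspection; disengaging returns it, marking it discarded if unpinned.
; Unpinning animates and destroys the pin before calling Dispell on the sigil.
; Sphere overlaps toggle outline overlay materials, while getter functions supply prompt, comment and UI data.
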(event `self.ReceiveBeginPlay`)

(event `self.Interact`
  (params (Interactor :type "Actor Object Reference"))
  (bind (_returnvalue_location _returnvalue_rotation) (`KismetMathLibrary.BreakTransform` (`self.GetTransform`)))
  (if (not (`self.Discarded`))
    (set `self.isBeingExamined` true)
    (message `/Game/ExportToBayou/BPI_Player.DisableMovement` Interactor true)
    (message `/Game/ExportToBayou/BPI_Player.SetIgnoreLookInput` Interactor true)
    (set `self.OriginalLocation` _returnvalue_location)
    (set `self.OriginalRotation` _returnvalue_rotation)
    (`self.K2_AttachToComponent` self (`PlayerCameraManager.TransformComponent` (`GameplayStatics.GetPlayerCameraManager` 0)) "None" "KeepWorld" "KeepWorld" "KeepWorld" true)
    (`KismetSystemLibrary.MoveComponentTo` (`self.DefaultSceneRoot`) (200.0 0.0 30.0) (struct) false false 0.3)
    (`GameplayStatics.PlaySoundAtLocation` (`self.ExamineSound`) (`self.K2_GetActorLocation` self) (struct) 1.0 1.0 0.0 null null null null)))

(event `self.Disengage`
  (params (Interactor :type "Actor Object Reference"))
  (set `self.isBeingExamined` false)
  (message `/Game/ExportToBayou/BPI_Player.DisableMovement` Interactor false)
  (message `/Game/ExportToBayou/BPI_Player.SetIgnoreLookInput` Interactor false)
  (`self.K2_DetachFromActor` self "KeepWorld" "KeepWorld" "KeepWorld")
  (`KismetSystemLibrary.MoveComponentTo` (`self.DefaultSceneRoot`) (`self.OriginalLocation`) (`self.OriginalRotation`) false false 0.3)
  (`GameplayStatics.PlaySoundAtLocation` (`self.ExamineSound`) (`self.K2_GetActorLocation` self) (struct) 1.0 1.0 0.0 null null null null)
  (if (`self.IsUnpinned`)
    (set `self.Discarded` true)
    (`MeshComponent.SetOverlayMaterial` (`self.Doll`) null)))

(event `self.FlipInspect`
  (if (`self.isBeingExamined`)
    (if (`self.IsTurned`)
      (set `self.TargetTurnRotation` (struct))
      (set `self.IsTurned` false)
      (else
        (set `self.TargetTurnRotation` (struct :`Yaw` 180.0))
        (set `self.IsTurned` true)))
    (`KismetSystemLibrary.MoveComponentTo` (`self.DefaultSceneRoot`) (200.0 0.0 30.0) (`self.TargetTurnRotation`))))

(event `/Game/ExportToBayou/BPI_Interactable.UnpinDoll`
  (if (not (`self.IsUnpinned`))
    (`KismetSystemLibrary.MoveComponentTo` (`self.Pin`) (`self.Unpin Location`) (struct :`Pitch` -50.0))
    (set `self.IsUnpinned` true)
    (`KismetSystemLibrary.Delay` 0.5) ; Nadja Yaps
    (`ActorComponent.K2_DestroyComponent` (`self.Pin`))
    (`self.EnableInput` (`GameplayStatics.GetPlayerCharacter` 0) (`GameplayStatics.GetPlayerController` 0))
    (`/Game/Karris_Flashlight/Blueprints/BP_ProtectionSymbol.Dispell` (`self.AssignedSigil`))))

(event `self.Sphere.OnComponentBeginOverlap`
  (params (OverlappedComponent :type "PrimitiveComponent Object Reference") (OtherActor :type "Actor Object Reference") (OtherComp :type "PrimitiveComponent Object Reference") (OtherBodyIndex :type Integer) (bFromSweep :type Boolean) (SweepResult :type "HitResult Structure (by ref)"))
  (if (`KismetSystemLibrary.DoesImplementInterface` OtherActor "/Game/ExportToBayou/BPI_Player.BPI_Player_C")
    (if (not (`self.Discarded`))
      (`MeshComponent.SetOverlayMaterial` (`self.Doll`) "/Game/ExportToBayou/M_OutlineMaterial.M_OutlineMaterial")
      (if (not (`self.IsUnpinned`))
        (`MeshComponent.SetOverlayMaterial` (`self.Pin`) "/Game/ExportToBayou/M_OutlineMaterial.M_OutlineMaterial")))))

(event `self.Sphere.OnComponentEndOverlap`
  (params (OverlappedComponent :type "PrimitiveComponent Object Reference") (OtherActor :type "Actor Object Reference") (OtherComp :type "PrimitiveComponent Object Reference") (OtherBodyIndex :type Integer))
  (if (`KismetSystemLibrary.DoesImplementInterface` OtherActor "/Game/ExportToBayou/BPI_Player.BPI_Player_C")
    (`MeshComponent.SetOverlayMaterial` (`self.Doll`) null)
    (if (not (`self.IsUnpinned`))
      (`MeshComponent.SetOverlayMaterial` (`self.Pin`) null))))

(event `/Game/ExportToBayou/BPI_Interactable.TalkedAbout`
  (params (TalkedAbout :type Boolean))
  (set `self.Has Been Commented` TalkedAbout))

(event `/Game/ExportToBayou/BPI_Interactable.TalkedAboutBack`
  (params (TalkedAboutBack :type Boolean))
  (set `self.Has Been Commented Back` TalkedAboutBack))

(fn `GetHoldDuration`
  (returns (Duration :type "Float (double-precision)"))
  (return 0.5))

(fn `GetInspectInfo`
  (returns (Name :type Text) (PlayerComment :type Text) (PlayerBackComment :type Text) (HasComment :type Boolean) (HasBackComment :type Boolean) (HasBeenCommented :type Boolean) (HasBeenCommentedBack :type Boolean) (FrontDialogueDuration :type "Float (double-precision)") (BackDialogueDuration :type "Float (double-precision)"))
  (return (`self.ItemName`) (`self.Player Comment`) (`self.Player Back Comment`) (`self.Has Comment`) (`self.Has Back Comment`) (`self.Has Been Commented`) (`self.Has Been Commented Back`) (`self.Front Dialogue Duration`) (`self.Back Dialogue Duration`)))

(fn `GetInteractionPrompt`
  (returns (Value :type Text))
  (return (select `bool` (`self.isBeingExamined`) :`false` "to open the door" :`true` "to close the door" :!type "Text")))

(fn `GetInteractionType`
  (returns (Type :type "/Game/ExportToBayou/E_InteractionInputType Enum"))
  (return (`self.InputType`)))

(fn `IsBeingInteractedWith?`
  (returns (IsInteracting :type Boolean))
  (return (`self.isBeingExamined`)))

(fn `IsDoll?`
  (returns (Dollness :type Boolean))
  (return true))

(fn `isInspectable?`
  (returns (isInspectObject :type Boolean))
  (return true))

(fn `SetAnimation`
  (returns (InteractAnimation :type "AnimMontage Object Reference"))
  (return (`self.InteractAnimation`)))

(fn `SetUI`
  (returns (DrawSize :type "Vector2D Structure") (UILocation :type "Vector Structure"))
  (return (`self.UIDrawSize`) (`SceneComponent.K2_GetComponentLocation` (`self.UI Render Point`))))

(fn `ShouldBeLookedAt`
  (returns (LookAtMe :type Boolean))
  (return true))

(fn `UserConstructionScript`)