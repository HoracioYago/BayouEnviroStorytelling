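; BP_ProtectionSymbol is a seal symbol that hides while the flashlight overlaps it and reappears afterwards unless it has been dispelled.
; Dispelling sets a flag, plays a seal-breaking sound at the symbol, then hides it after a delay.
; An AtticSigil flag selects what follows: the assigned attic door opens its stairs, or the assigned door creepily opens after a further delay.
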(event `Flashlight_Overlap`
  ;[1 1 1] Disappear
  (`SceneComponent.SetVisibility` (`self.Symbol`) false false))

(event `End_Flashlight_Overlap`
  ;[1 1 1] Reappear
  (if (not (`self.Dispelled`))
    (`SceneComponent.SetVisibility` (`self.Symbol`) true false)))

(event `/Game/ExportToBayou/BPI_ProtectionCircle.Dispell`
  ;[0.776 0 0.184] Dispell
  (if (`self.AtticSigil`)
    (set `self.Dispelled` true)
    (`GameplayStatics.PlaySoundAtLocation` "/Game/Sounds/Seal_Breaking.Seal_Breaking" (`SceneComponent.K2_GetComponentLocation` (`self.Symbol`)) (struct) 1.0 1.0 0.0 null null null null)
    (`KismetSystemLibrary.Delay` 2.0)
    (`SceneComponent.SetVisibility` (`self.Symbol`) false false)
    (`/Game/ExportToBayou/BP_AtticStairs.OpenAtticStairs` (`self.AssignedAtticDoor`))
    (else
      (set `self.Dispelled` true)
      (`GameplayStatics.PlaySoundAtLocation` "/Game/Sounds/Seal_Breaking.Seal_Breaking" (`SceneComponent.K2_GetComponentLocation` (`self.Symbol`)) (struct) 1.0 1.0 0.0 null null null null)
      (`KismetSystemLibrary.Delay` 2.0)
      (`SceneComponent.SetVisibility` (`self.Symbol`) false false)
      (`KismetSystemLibrary.Delay` 2.0)
      (`/Game/ExportToBayou/BP_Door.CreepyOpen` (`self.AssignedDoor`)))))

(fn `UserConstructionScript`)